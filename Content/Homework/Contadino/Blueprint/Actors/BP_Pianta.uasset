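; BP_Pianta is a plant actor that ripens after a timer and can then be harvested by the farmer, BP_Contadino.
; When the maturation delay ends, it becomes harvestable, takes the Pianta.Matura gameplay tag and switches its mesh to a green material.
; Its Interact event, once ripe, increments the farmer's harvested count, resets its indexed slot in BP_ZonaPiante's SlotPiantati array and destroys the plant.
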(event `self.ReceiveBeginPlay`
  (`KismetSystemLibrary.Delay` (`self.TimerMaturazione`))
  (set `self.Raccoglibile` true)
  (bind _output_get (set `self.QueryTag` (struct :`TagName` "Pianta.Matura")))
  (set `self.PiantaGameplayTags` (`BlueprintGameplayTagLibrary.MakeGameplayTagContainerFromTag` _output_get))
  (`PrimitiveComponent.SetMaterial` (`self.Mesh`) 0 "/Game/Homework/Contadino/Material/Instances/MI_Green.MI_Green"))

(event `/Game/Homework/Contadino/Blueprint/Interface/BPI_Interactable.Interact`
  (params (Requester :type "Actor Object Reference"))
  (if (`self.Raccoglibile`)
    (`KismetSystemLibrary.IsObjectOfSoftClass` Requester "/Game/Homework/Contadino/Blueprint/BP_Contadino.BP_Contadino_C"
      (:`True`
        (bind _asbp_contadino (cast `/Game/Homework/Contadino/Blueprint/BP_Contadino` Requester))
        (bind _result (`/Engine/EditorBlueprintResources/StandardMacros.IncrementInt` (`/Game/Homework/Contadino/Blueprint/BP_Contadino.PianteRaccolte` _asbp_contadino))
          (:`  `
            (set `/Game/Homework/Contadino/Blueprint/BP_Contadino.PianteRaccolte` _result _asbp_contadino)
            (bind _returnvalue (`GameplayStatics.GetActorOfClass` "/Game/Homework/Contadino/Blueprint/Actors/BP_ZonaPiante.BP_ZonaPiante_C"))
            (`KismetArrayLibrary.Array_Set` (`/Game/Homework/Contadino/Blueprint/Actors/BP_ZonaPiante.SlotPiantati` _returnvalue) (`self.ZoneIndex`))
            (`self.K2_DestroyActor`)))))))

(fn `UserConstructionScript`)