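; BP_Torretta is an AI turret with three states: alert (Allerta), active (Attiva) and inactive (Disattiva).
; On BeginPlay it applies its initial state through ChangeState, which writes the State key to the Blackboard and stores the value locally.
; ChangeState then calls ChangeColor to tint the base and cannon meshes cyan, red or gray to match.
; Shoot is a placeholder that only prints a debug message, with firing still marked TODO.
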(event `self.ReceiveBeginPlay`
  (`self.ChangeState` (`self.State`)))

(fn `ChangeColor`
  (params (NewMaterialInstance :type "MaterialInstance Object Reference"))
  (`PrimitiveComponent.SetMaterial` (`self.MeshBase`) 0 NewMaterialInstance)
  (`PrimitiveComponent.SetMaterial` (`self.MeshCannone`) 0 NewMaterialInstance))

(fn `ChangeState`
  (params (NewState :type "/Game/Homework/Torretta/Blueprint/BP_TorrettaStates Enum" :default "NewEnumerator0"))
  (`BlackboardComponent.SetValueAsEnum` (`AIBlueprintHelperLibrary.GetBlackboard` null) "State" NewState)
  (bind _output_get (set `self.State` NewState))
  (switch `/Game/Homework/Torretta/Blueprint/BP_TorrettaStates` _output_get
    (:`NewEnumerator0`
      (`self.ChangeColor` "/Game/Homework/Torretta/Material/MI_Cyan.MI_Cyan"))
    (:`NewEnumerator1`
      (`self.ChangeColor` "/Game/Homework/Torretta/Material/MI_Red.MI_Red"))
    (:`NewEnumerator2`
      (`self.ChangeColor` "/Game/Homework/Torretta/Material/MI_Gray.MI_Gray"))))

(fn `Shoot`
  ; TODO fai sparare la torretta
  (`KismetSystemLibrary.PrintString` "Shot!" true true (struct :`G` 0.66 :`B` 1.0 :`A` 1.0) 0.5 "Turret"))

(fn `UserConstructionScript`)