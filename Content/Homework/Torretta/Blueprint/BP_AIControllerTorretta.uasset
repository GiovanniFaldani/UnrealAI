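; AI controller for the BP_Torretta turret, running BT_Torretta and seeding its blackboard State from the turret on possess.
; AI perception of actors tagged "Bersaglio" switches the turret's state and stores the blackboard Target.
; Losing sight starts a memory timer, kept on the turret and cancelled on re-sighting, which clears the target and returns the turret to inactive when it expires.
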(event `self.ReceivePossess`
  (params (PossessedPawn :type "Pawn Object Reference"))
  (`self.RunBehaviorTree` "/Game/Homework/Torretta/Blueprint/BehaviorTree/BT_Torretta.BT_Torretta")
  ; Init State
  (bind _asbp_torretta (cast `/Game/Homework/Torretta/Blueprint/BP_Torretta` PossessedPawn))
  (`BlackboardComponent.SetValueAsEnum` (`AIBlueprintHelperLibrary.GetBlackboard` null) "State" (`/Game/Homework/Torretta/Blueprint/BP_Torretta.State` _asbp_torretta)))

(event `self.AIPerception.OnTargetPerceptionUpdated`
  (params (Actor :type "Actor Object Reference") (Stimulus :type "AIStimulus Structure"))
  (bind _output_get (set `self.TargetActor` Actor))
  (if (`self.ActorHasTag` _output_get "Bersaglio")
    (if Stimulus_bSuccessfullySensed
      (`KismetSystemLibrary.PrintString` "Found a target!" true true (struct :`R` 1.0 :`G` 0.019885 :`B` 0.983437 :`A` 1.0) 2.0 "TurretController")
      ; Bersaglio in vista
      (bind _asbp_torretta (cast `/Game/Homework/Torretta/Blueprint/BP_Torretta` (`self.K2_GetPawn`)))
      (`KismetSystemLibrary.K2_ClearAndInvalidateTimerHandle` (`/Game/Homework/Torretta/Blueprint/BP_Torretta.MemoryTimerHandle` _asbp_torretta))
      (`/Game/Homework/Torretta/Blueprint/BP_Torretta.ChangeState` _asbp_torretta "NewEnumerator1")
      (`BlackboardComponent.SetValueAsObject` (`AIBlueprintHelperLibrary.GetBlackboard` null) "Target" (`self.TargetActor`))
      (else
        (`KismetSystemLibrary.PrintString` "Lost sight of Target!" true true (struct :`R` 1.0 :`G` 0.019885 :`B` 0.983437 :`A` 1.0) 2.0 "TurretController")
        ; Bersaglio non in vista
        (bind _asbp_torretta_2 (cast `/Game/Homework/Torretta/Blueprint/BP_Torretta` (`self.K2_GetPawn`)))
        (bind _returnvalue (`KismetSystemLibrary.K2_SetTimerDelegate` (delegate `ForgetTarget`) (`/Game/Homework/Torretta/Blueprint/BP_Torretta.MemoryTime` _asbp_torretta_2)))
        (set `/Game/Homework/Torretta/Blueprint/BP_Torretta.MemoryTimerHandle` _returnvalue _asbp_torretta_2)))))

(event `ForgetTarget`
  ; Bersaglio non in vista
  (`BlackboardComponent.ClearValue` (`AIBlueprintHelperLibrary.GetBlackboard` null) "Target")
  (`/Game/Homework/Torretta/Blueprint/BP_Torretta.ChangeState` (stale `self.AIPerception.OnTargetPerceptionUpdated` _asbp_torretta_2) "NewEnumerator0")
  (`KismetSystemLibrary.PrintString` "Returning inactive..." true true (struct :`R` 1.0 :`G` 0.019885 :`B` 0.983437 :`A` 1.0) 2.0 "TurretController"))

(fn `UserConstructionScript`)